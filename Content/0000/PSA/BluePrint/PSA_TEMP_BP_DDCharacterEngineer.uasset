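; Temporary engineer character Blueprint that drives and debugs a PlayerMap for tracking the player's position on a map.
; BeginPlay initializes the map with the character, prints its width and height, and starts a looping timer that prints the character's location in map coordinates.
; Non-zero move input notifies PlayerMap that the player moved.
; Other input, overlap and tick events are empty stubs.
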(event Input|EnhancedActionEvents|EnhancedInputActionIA_Player_Move
  (params (ActionValue :type Vector%202D%20Structure) (ElapsedSeconds :type Float%20%28double-precision%29) (TriggeredSeconds :type Float%20%28double-precision%29) (InputAction :type Input%20Action%20Object%20Reference :default "/Game/0000/LJW/Input/IA_Player_Move.IA_Player_Move"))
  (bind (_x _y) (Math|Vector2D|BreakVector2D ActionValue))
  (if (or (!= _x 0.0) (!= _y 0.0))
    (Default|OnPlayerMoved (Variables|Default|GetPlayerMap))))

(event Input|EnhancedActionEvents|EnhancedInputActionIA_Player_BackMove
  (params (ActionValue :type Boolean) (ElapsedSeconds :type Float%20%28double-precision%29) (TriggeredSeconds :type Float%20%28double-precision%29) (InputAction :type Input%20Action%20Object%20Reference :default "/Game/0000/LJW/Input/IA_Player_BackMove.IA_Player_BackMove")))

(event Input|EnhancedActionEvents|EnhancedInputActionIA_Player_Sprint
  (params (ActionValue :type Boolean) (ElapsedSeconds :type Float%20%28double-precision%29) (TriggeredSeconds :type Float%20%28double-precision%29) (InputAction :type Input%20Action%20Object%20Reference :default "/Game/0000/LJW/Input/IA_Player_Sprint.IA_Player_Sprint")))

(event Input|EnhancedActionEvents|EnhancedInputActionIA_Player_Jump
  (params (ActionValue :type Boolean) (ElapsedSeconds :type Float%20%28double-precision%29) (TriggeredSeconds :type Float%20%28double-precision%29) (InputAction :type Input%20Action%20Object%20Reference :default "/Game/0000/LJW/Input/IA_Player_Jump.IA_Player_Jump")))

(event EventBeginPlay
  (bind _playermap (Variables|Default|GetPlayerMap))
  (Default|InitializeMap _playermap self)
  (Development|PrintString (Utilities|String|Append "Width:" (Utilities|String|ToString(Float) (Default|GetMapWidth _playermap)) " Height:" (Utilities|String|ToString(Float) (Default|GetMapHeight _playermap))) true true "(R=0.000000,G=1.000000,B=0.000000,A=1.000000)" 1e+01)
  (Utilities|Time|SetTimerbyFunctionName 0 "Print Location" 1.0 true))

(event Collision|EventActorBeginOverlap
  (params (OtherActor :type Actor%20Object%20Reference)))

(event EventTick
  (params (DeltaSeconds :type Float%20%28single-precision%29)))

(fn ConstructionScript)

(fn PrintLocation
  (Development|PrintString (Utilities|String|ToString(Vector2d) (Default|ConvertLocationtoMapLocation (Variables|Default|GetPlayerMap) (Transformation|GetActorLocation))) true true "(R=0.000000,G=0.660000,B=1.000000,A=1.000000)" 1.0))