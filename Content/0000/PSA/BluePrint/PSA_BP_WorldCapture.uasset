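; World capture actor that frames a rectangular area of the level with an orthographic scene capture, apparently for a minimap.
; The construction script centers it between the UpperLeft and LowerRight actors, keeping its height, and sets OrthoWidth to the larger X/Y span.
; AllActors and ShowOnlyList would restrict capture to "MiniMap"-tagged static meshes and DDEnemyBase children, but their calls are disconnected.
; The event graph is empty.
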(event EventBeginPlay)

(event Collision|EventActorBeginOverlap
  (params (OtherActor :type Actor%20Object%20Reference)))

(event EventTick
  (params (DeltaSeconds :type Float%20%28single-precision%29)))

(fn ConstructionScript
  (bind _lowerright (Variables|Default|GetLowerRight))
  (bind _upperleft (Variables|Default|GetUpperLeft))
  (bind _lowerright_2 (Variables|Default|GetLowerRight))
  (bind _upperleft_2 (Variables|Default|GetUpperLeft))
  (bind _returnvalue (Transformation|GetActorLocation _upperleft))
  (bind _returnvalue_2 (Transformation|GetActorLocation _lowerright))
  (bind _returnvalue_3 (Transformation|GetActorLocation _lowerright_2))
  (bind _returnvalue_4 (Transformation|GetActorLocation _upperleft_2))
  (bind (_x _y) (Math|Vector|BreakVector _returnvalue_3))
  (bind (_x_2 _y_2) (Math|Vector|BreakVector _returnvalue_4))
  (bind _returnvalue_5 (- _returnvalue_2 _returnvalue))
  (bind _returnvalue_6 (/ _returnvalue_5 2.0))
  (bind _returnvalue_7 (+ _returnvalue _returnvalue_6))
  (bind (_x_3 _y_3) (Math|Vector|BreakVector _returnvalue_7))
  (Utilities|IsValid (Variables|Default|GetUpperLeft)
    (:Is%20Valid
      (Utilities|IsValid (Variables|Default|GetLowerRight)
        (:Is%20Valid
          (Transformation|SetActorLocation (Math|Vector|MakeVector _x_3 _y_3 (.Z (Math|Vector|BreakVector (Transformation|GetActorLocation)))) false true)
          (Variables|/Script/Engine.SceneCaptureComponent2D|SetOrthoWidth (Variables|Default|GetSceneCapture) (Math|Float|Max(Float) (Math|Float|Absolute(Float) (- _x _x_2)) (Math|Float|Absolute(Float) (- _y _y_2)))))))))

(fn ShowOnlyList
  (for _array_element (Variables|Default|GetAllActor)
    ;[1 1 1] MiniMap
    (bind _asstatic_mesh_actor (Utilities|Casting|CastToStaticMeshActor _array_element))
    (if (Components|ComponentHasTag (Variables|/Script/Engine.StaticMeshActor|GetStaticMeshComponent _asstatic_mesh_actor) "MiniMap")
      (Utilities|Array|Add (Variables|Default|GetShowActor) _array_element)
      (else
        ;[1 1 1] Enemy
        (if (Utilities|ClassIsChildOf (Utilities|GetClass _array_element) "/Script/ProjectD.DDEnemyBase")
          (Utilities|Array|Add (Variables|Default|GetShowActor) _array_element)))))
  ;[1 1 1] Show Actor
  (Variables|/Script/Engine.SceneCaptureComponent|SetShowOnlyActors (Variables|Default|GetSceneCapture) (Variables|Default|GetShowActor)))

(fn AllActors
  (Utilities|Array|Clear (Variables|Default|GetAllActor))
  (bind _outactors (Actor|GetAllActorsOfClass "/Script/Engine.Actor"))
  (Variables|Default|SetAllActor _outactors))