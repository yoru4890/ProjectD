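; Engineer character Blueprint with a hard-bound key 5 hitscan attack, apparently for testing.
; Pressing 5 runs a line trace forward from the follow camera on a custom trace channel, with debug drawing enabled.
; If the hit actor derives from DDEnemyBase, it receives a small fixed amount of piercing damage.
; The Blueprint adds no other active logic.
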(event EventBeginPlay
  (|CallParentFunction) ; This node is disabled and will not be called.\nDrag off pins to build functionality.
)

(event Collision|EventActorBeginOverlap
  (params (OtherActor :type Actor%20Object%20Reference))
  (|CallParentFunction OtherActor) ; This node is disabled and will not be called.\nDrag off pins to build functionality.
)

(event EventTick
  (params (DeltaSeconds :type Float%20%28single-precision%29))
  (|CallParentFunction DeltaSeconds) ; This node is disabled and will not be called.\nDrag off pins to build functionality.
)

(event Input|KeyboardEvents|5
  (params (Key :type Key%20Structure :default "None"))
  (bind _followcamera (Variables|Default|GetFollowCamera))
  (bind _returnvalue (Transformation|GetWorldLocation _followcamera))
  (:Pressed
    (bind (_outhit _returnvalue_2) (Collision|LineTraceByChannel _returnvalue (+ _returnvalue (* (Math|Vector|GetForwardVector _followcamera) 1e+04)) "TraceTypeQuery4" false 0 "ForDuration"))
    (if _returnvalue_2
      (if (Utilities|ClassIsChildOf (Utilities|GetClass (.HitActor (Collision|BreakHitResult _outhit))) "/Script/ProjectD.DDEnemyBase")
        (Game|Damage|ApplyDamage (.HitActor (Collision|BreakHitResult _outhit)) 5.0 0 0 "/Script/ProjectD.PiercingDamageType")))))

(fn ConstructionScript
  (|CallParentFunction))