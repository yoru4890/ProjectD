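; Temporary child of the DD engineer character Blueprint, used as a test harness for save data and the building system.
; BeginPlay calls the parent, caches DDPlayerState and creates a "Temp" save file.
; The 0 key has the game instance's BuildingManager handle building pools for a level change, then initializes BuildSystem's grid build manager.
; Leftover debug chains for building unlocks, slot save/load, autosave and like points are disconnected and never run.
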(event EventBeginPlay
  (|CallParentFunction)
  (bind _asddplayer_state (Utilities|Casting|CastToDDPlayerState (Game|GetPlayerState 0)))
  (Variables|Default|SetAs%20DDPlayer%20State _asddplayer_state)
  (Class|DDPlayerState|CreateSaveFile (Variables|Default|GetAs%20DDPlayer%20State) "Temp"))

(event Collision|EventActorBeginOverlap
  (params (OtherActor :type Actor%20Object%20Reference))
  (|CallParentFunction OtherActor) ; This node is disabled and will not be called.\nDrag off pins to build functionality.
)

(event EventTick
  (params (DeltaSeconds :type Float%20%28single-precision%29))
  (|CallParentFunction DeltaSeconds) ; This node is disabled and will not be called.\nDrag off pins to build functionality.
)

(event Input|KeyboardEvents|9
  (params (Key :type Key%20Structure :default "None")))

(event Input|KeyboardEvents|0
  (params (Key :type Key%20Structure :default "None"))
  (:Pressed
    (bind _asddgame_instance (Utilities|Casting|CastToDDGameInstance (Game|GetGameInstance)))
    (Class|DDBuildingManager|HandleBuildingPoolsonLevelChange (Class|DDGameInstance|GetBuildingManager _asddgame_instance))
    (Class|DDBuildComponent|InitGridBuildManager (Variables|Default|GetBuildSystem))))

(event Input|KeyboardEvents|7
  (params (Key :type Key%20Structure :default "None")))

(event Input|KeyboardEvents|8
  (params (Key :type Key%20Structure :default "None")))

(event Input|KeyboardEvents|O
  (params (Key :type Key%20Structure :default "None")))

(event Input|KeyboardEvents|5
  (params (Key :type Key%20Structure :default "None")))

(event Input|KeyboardEvents|6
  (params (Key :type Key%20Structure :default "None")))

(event Input|KeyboardEvents|4
  (params (Key :type Key%20Structure :default "None")))

(fn ConstructionScript
  (|CallParentFunction))