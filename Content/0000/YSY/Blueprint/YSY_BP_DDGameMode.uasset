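; Game mode Blueprint that boots the game into a title menu and provides stage start-up.
; BeginPlay adds a loading widget, starts non-blocking streaming of the intro level, switches to UI-only input with a cursor, then immediately clears all widgets and shows the title menu.
; InitStage passes the stage index to the game instance's WaveManager, shows the player controller's main widget, and switches to game-only input without a cursor.
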(event EventBeginPlay
  (bind _returnvalue (Game|GetPlayerController 0))
  (bind _returnvalue_2 (UserInterface|CreateWidget "/Game/0000/YSY/LevelStreamingTest/Widget/YSY_WBP_MyLoading.YSY_WBP_MyLoading_C"))
  (bind _output_get (Variables|Default|SetLoadingWidget _returnvalue_2))
  (UserInterface|Viewport|AddtoViewport _output_get 0)
  ;[1 1 1] 2. 타이틀메뉴
  (Class|GameplayStatics|LoadStreamLevelbySoftObjectPtr "/Game/0000/YSY/LevelStreamingTest/Lv_YSY_Intro.Lv_YSY_Intro" true false)
  (Input|SetInputModeUIOnly _returnvalue 0 "DoNotLock" false)
  (Variables|/Script/Engine.PlayerController|SetbShowMouseCursor _returnvalue true)
  (Viewport|RemoveAllWidgets)
  (bind _returnvalue_3 (UserInterface|CreateWidget "/Game/0000/YSY/LevelStreamingTest/Widget/LevelST_YSY_WBP_TitleMenu.LevelST_YSY_WBP_TitleMenu_C"))
  (bind _output_get_2 (Variables|Default|SetTitleWidget _returnvalue_3))
  (UserInterface|Viewport|AddtoViewport _output_get_2 0))

(event EventTick
  (params (DeltaSeconds :type Float%20%28single-precision%29)))

(fn ConstructionScript)

(fn InitStage
  (params (StageIndex :type Integer))
  (bind _returnvalue (Game|GetPlayerController 0))
  (bind _asddgame_instance (Utilities|Casting|CastToDDGameInstance (Game|GetGameInstance)))
  (Class|DDWaveManager|InitStage (Class|DDGameInstance|GetWaveManager _asddgame_instance) StageIndex)
  (bind _asddplayer_controller (Utilities|Casting|CastToDDPlayerController (Game|GetPlayerController 0)))
  (Class|DDPlayerController|ShowMainWidget _asddplayer_controller)
  (Input|SetInputModeGameOnly _returnvalue false)
  (Variables|/Script/Engine.PlayerController|SetbShowMouseCursor _returnvalue false))