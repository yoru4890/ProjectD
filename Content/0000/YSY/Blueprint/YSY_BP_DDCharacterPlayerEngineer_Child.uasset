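; Child Blueprint of the engineer player character that binds number keys to what appear to be damage and debuff tests on enemies.
; Keys 1-3 apply Hacking, Piercing or Corrosion damage to a single YSY_BP_EnemyBase found by class lookup.
; Key 4 line-traces from the follow camera with debug drawing, applying point damage only on an exact DDEnemyBase class match.
; Keys 5-6 apply timed Slow or DamageIncrease debuffs to every DDEnemyBase.
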(event EventBeginPlay
  (|CallParentFunction) ; This node is disabled and will not be called.\nDrag off pins to build functionality.
)

(event Collision|EventActorBeginOverlap
  (params (OtherActor :type Actor%20Object%20Reference))
  (|CallParentFunction OtherActor) ; This node is disabled and will not be called.\nDrag off pins to build functionality.
)

(event EventTick
  (params (DeltaSeconds :type Float%20%28single-precision%29))
  (|CallParentFunction DeltaSeconds) ; This node is disabled and will not be called.\nDrag off pins to build functionality.
)

(event Input|KeyboardEvents|4
  (params (Key :type Key%20Structure :default "None"))
  (bind _followcamera (Variables|Default|GetFollowCamera))
  (bind _returnvalue (Transformation|GetWorldLocation _followcamera))
  (:Pressed
    (bind (_outhit _returnvalue_2) (Collision|LineTraceByChannel _returnvalue (+ _returnvalue (* (Math|Vector|GetForwardVector _followcamera) 1e+04)) "TraceTypeQuery4" false 0 "ForDuration"))
    (if _returnvalue_2
      (if (== (Utilities|GetClass (.HitActor (Collision|BreakHitResult _outhit))) "/Script/ProjectD.DDEnemyBase")
        (Game|Damage|ApplyPointDamage (.HitActor (Collision|BreakHitResult _outhit)) 5.0 (.Normal (Collision|BreakHitResult _outhit)) _outhit)))))

(event Input|KeyboardEvents|1
  (params (Key :type Key%20Structure :default "None"))
  (:Pressed
    (bind _returnvalue (Actor|GetActorOfClass "/Game/0000/YSY/Blueprint/YSY_BP_EnemyBase.YSY_BP_EnemyBase_C"))
    (Game|Damage|ApplyDamage _returnvalue 1.0 0 0 "/Script/ProjectD.HackingDamageType")))

(event Input|KeyboardEvents|2
  (params (Key :type Key%20Structure :default "None"))
  (:Pressed
    (bind _returnvalue (Actor|GetActorOfClass "/Game/0000/YSY/Blueprint/YSY_BP_EnemyBase.YSY_BP_EnemyBase_C"))
    (Game|Damage|ApplyDamage _returnvalue 1.0 0 0 "/Script/ProjectD.PiercingDamageType")))

(event Input|KeyboardEvents|3
  (params (Key :type Key%20Structure :default "None"))
  (:Pressed
    (bind _returnvalue (Actor|GetActorOfClass "/Game/0000/YSY/Blueprint/YSY_BP_EnemyBase.YSY_BP_EnemyBase_C"))
    (Game|Damage|ApplyDamage _returnvalue 1.0 0 0 "/Script/ProjectD.CorrosionDamageType")))

(event Input|KeyboardEvents|5
  (params (Key :type Key%20Structure :default "None"))
  (:Pressed
    (bind _outactors (Actor|GetAllActorsOfClass "/Script/ProjectD.DDEnemyBase"))
    (for _array_element _outactors
      (Class|DDEnemyBase|ApplyDebuff _array_element "Slow" 5.0 0.5))))

(event Input|KeyboardEvents|6
  (params (Key :type Key%20Structure :default "None"))
  (:Pressed
    (bind _outactors (Actor|GetAllActorsOfClass "/Script/ProjectD.DDEnemyBase"))
    (for _array_element _outactors
      (Class|DDEnemyBase|ApplyDebuff _array_element "DamageIncrease" 5.0 1.5))))

(fn ConstructionScript
  (|CallParentFunction))