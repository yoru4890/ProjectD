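; BP_BGM is a background music Blueprint that plays 2D music for the game.
; On BeginPlay it spawns a 2D sound with a climax track, then immediately switches that component to 01Electric and plays it.
; Separate events select the start or in-game track from BGMList into PlayingBGM.
; BGM_Play plays that selection as a new 2D sound, independently of the BeginPlay component, which it never stops.
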(event Custom|BGM_Start
  (Variables|Default|SetPlayingBGM (.StartBGM (Utilities|Struct|BreakStruct_BGM (Variables|Default|GetBGMList)))))

(event Custom|BGM_Ingame
  (Variables|Default|SetPlayingBGM (.InGameBGM (Utilities|Struct|BreakStruct_BGM (Variables|Default|GetBGMList)))))

(event Custom|BGM_Play
  (Audio|PlaySound2D (Variables|Default|GetPlayingBGM) 1.0 1.0 0.0 0 0))

(event EventBeginPlay
  (bind _returnvalue (Audio|SpawnSound2D "/Game/0000/LJW/Sounds/BGM/WAV_Colossal_Hybrid_Action_Climax_Full.WAV_Colossal_Hybrid_Action_Climax_Full" 1.0 1.0 0.0 0))
  (Audio|Components|Audio|SetSound _returnvalue "/Game/BallisticsVFX/SFX/Impacts/Electric/01-Electric.01-Electric")
  (Audio|Components|Audio|Play _returnvalue 0.0))

(fn ConstructionScript)