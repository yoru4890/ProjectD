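; Respawn wall actor that encloses a volume with six box triggers and respawns player characters that touch its boundary.
; The construction script positions and flattens the boxes into the faces of a cuboid sized by RespawnBoxSize.
; Overlap events from all six boxes share one path that casts the other actor to DDCharacterPlayer and calls its Spawn function.
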(event OnComponentBeginOverlap(Box_Front)
  (params (OverlappedComponent :type Primitive%20Component%20Object%20Reference) (OtherActor :type Actor%20Object%20Reference) (OtherComp :type Primitive%20Component%20Object%20Reference) (OtherBodyIndex :type Integer) (bFromSweep :type Boolean) (SweepResult :type Hit%20Result%20Structure%20%28by%20ref%29))
  (Variables|Default|SetOther%20Actor OtherActor)
  (bind _asddcharacter_player (Utilities|Casting|CastToDDCharacterPlayer (Variables|Default|GetOther%20Actor)))
  (Utilities|IsValid _asddcharacter_player
    (:Is%20Valid
      (Class|DDCharacterPlayer|Spawn _asddcharacter_player))))

(event OnComponentBeginOverlap(Box_Back)
  (params (OverlappedComponent :type Primitive%20Component%20Object%20Reference) (OtherActor :type Actor%20Object%20Reference) (OtherComp :type Primitive%20Component%20Object%20Reference) (OtherBodyIndex :type Integer) (bFromSweep :type Boolean) (SweepResult :type Hit%20Result%20Structure%20%28by%20ref%29))
  (Variables|Default|SetOther%20Actor OtherActor)
  (bind _asddcharacter_player (Utilities|Casting|CastToDDCharacterPlayer (Variables|Default|GetOther%20Actor)))
  (Utilities|IsValid _asddcharacter_player
    (:Is%20Valid
      (Class|DDCharacterPlayer|Spawn _asddcharacter_player))))

(event OnComponentBeginOverlap(Box_Left)
  (params (OverlappedComponent :type Primitive%20Component%20Object%20Reference) (OtherActor :type Actor%20Object%20Reference) (OtherComp :type Primitive%20Component%20Object%20Reference) (OtherBodyIndex :type Integer) (bFromSweep :type Boolean) (SweepResult :type Hit%20Result%20Structure%20%28by%20ref%29))
  (Variables|Default|SetOther%20Actor OtherActor)
  (bind _asddcharacter_player (Utilities|Casting|CastToDDCharacterPlayer (Variables|Default|GetOther%20Actor)))
  (Utilities|IsValid _asddcharacter_player
    (:Is%20Valid
      (Class|DDCharacterPlayer|Spawn _asddcharacter_player))))

(event OnComponentBeginOverlap(Box_Right)
  (params (OverlappedComponent :type Primitive%20Component%20Object%20Reference) (OtherActor :type Actor%20Object%20Reference) (OtherComp :type Primitive%20Component%20Object%20Reference) (OtherBodyIndex :type Integer) (bFromSweep :type Boolean) (SweepResult :type Hit%20Result%20Structure%20%28by%20ref%29))
  (Variables|Default|SetOther%20Actor OtherActor)
  (bind _asddcharacter_player (Utilities|Casting|CastToDDCharacterPlayer (Variables|Default|GetOther%20Actor)))
  (Utilities|IsValid _asddcharacter_player
    (:Is%20Valid
      (Class|DDCharacterPlayer|Spawn _asddcharacter_player))))

(event OnComponentBeginOverlap(Box_Top)
  (params (OverlappedComponent :type Primitive%20Component%20Object%20Reference) (OtherActor :type Actor%20Object%20Reference) (OtherComp :type Primitive%20Component%20Object%20Reference) (OtherBodyIndex :type Integer) (bFromSweep :type Boolean) (SweepResult :type Hit%20Result%20Structure%20%28by%20ref%29))
  (Variables|Default|SetOther%20Actor OtherActor)
  (bind _asddcharacter_player (Utilities|Casting|CastToDDCharacterPlayer (Variables|Default|GetOther%20Actor)))
  (Utilities|IsValid _asddcharacter_player
    (:Is%20Valid
      (Class|DDCharacterPlayer|Spawn _asddcharacter_player))))

(event OnComponentBeginOverlap(Box_Bottom)
  (params (OverlappedComponent :type Primitive%20Component%20Object%20Reference) (OtherActor :type Actor%20Object%20Reference) (OtherComp :type Primitive%20Component%20Object%20Reference) (OtherBodyIndex :type Integer) (bFromSweep :type Boolean) (SweepResult :type Hit%20Result%20Structure%20%28by%20ref%29))
  (Variables|Default|SetOther%20Actor OtherActor)
  (bind _asddcharacter_player (Utilities|Casting|CastToDDCharacterPlayer (Variables|Default|GetOther%20Actor)))
  (Utilities|IsValid _asddcharacter_player
    (:Is%20Valid
      (Class|DDCharacterPlayer|Spawn _asddcharacter_player))))

(event EventBeginPlay)

(event Collision|EventActorBeginOverlap
  (params (OtherActor :type Actor%20Object%20Reference)))

(event EventTick
  (params (DeltaSeconds :type Float%20%28single-precision%29)))

(fn ConstructionScript
  (bind _respawn_box_size (Variables|Default|GetRespawn%20Box%20Size))
  (bind _respawn_box_size_2 (Variables|Default|GetRespawn%20Box%20Size))
  (bind _respawn_box_size_3 (Variables|Default|GetRespawn%20Box%20Size))
  (bind _respawn_box_size_4 (Variables|Default|GetRespawn%20Box%20Size))
  (bind _respawn_box_size_5 (Variables|Default|GetRespawn%20Box%20Size))
  (bind _respawn_box_size_6 (Variables|Default|GetRespawn%20Box%20Size))
  (Utilities|FlowControl|Sequence
    (:then_0
      (Transformation|SetRelativeLocation (Variables|Default|GetBox_Front) (Math|Vector|MakeVector (/ (.x (Variables|Default|GetRespawn%20Box%20Size)) 2.0) 0.0 0.0) false false)
      (Components|Box|SetBoxExtent (Variables|Default|GetBox_Front) (Math|Vector|MakeVector 1.0 (/ (.y _respawn_box_size) 2.0) (/ (.z _respawn_box_size) 2.0)) true))
    (:then_1
      (Transformation|SetRelativeLocation (Variables|Default|GetBox_Back) (Math|Vector|MakeVector (* (/ (.x (Variables|Default|GetRespawn%20Box%20Size)) 2.0) -1.0) 0.0 0.0) false false)
      (Components|Box|SetBoxExtent (Variables|Default|GetBox_Back) (Math|Vector|MakeVector 1.0 (/ (.y _respawn_box_size_2) 2.0) (/ (.z _respawn_box_size_2) 2.0)) true))
    (:then_2
      (Transformation|SetRelativeLocation (Variables|Default|GetBox_Right) (Math|Vector|MakeVector 0.0 (/ (.y (Variables|Default|GetRespawn%20Box%20Size)) 2.0) 0.0) false false)
      (Components|Box|SetBoxExtent (Variables|Default|GetBox_Right) (Math|Vector|MakeVector (/ (.x _respawn_box_size_3) 2.0) 1.0 (/ (.z _respawn_box_size_3) 2.0)) true))
    (:then_3
      (Transformation|SetRelativeLocation (Variables|Default|GetBox_Left) (Math|Vector|MakeVector 0.0 (* (/ (.y (Variables|Default|GetRespawn%20Box%20Size)) 2.0) -1.0) 0.0) false false)
      (Components|Box|SetBoxExtent (Variables|Default|GetBox_Left) (Math|Vector|MakeVector (/ (.x _respawn_box_size_4) 2.0) 1.0 (/ (.z _respawn_box_size_4) 2.0)) true))
    (:then_4
      (Transformation|SetRelativeLocation (Variables|Default|GetBox_Top) (Math|Vector|MakeVector 0.0 0.0 (/ (.z (Variables|Default|GetRespawn%20Box%20Size)) 2.0)) false false)
      (Components|Box|SetBoxExtent (Variables|Default|GetBox_Top) (Math|Vector|MakeVector (/ (.x _respawn_box_size_6) 2.0) (/ (.y _respawn_box_size_6) 2.0) 1.0) true))
    (:then_5
      (Transformation|SetRelativeLocation (Variables|Default|GetBox_Bottom) (Math|Vector|MakeVector 0.0 0.0 (* (/ (.z (Variables|Default|GetRespawn%20Box%20Size)) 2.0) -1.0)) false false)
      (Components|Box|SetBoxExtent (Variables|Default|GetBox_Bottom) (Math|Vector|MakeVector (/ (.x _respawn_box_size_5) 2.0) (/ (.y _respawn_box_size_5) 2.0) 0.0) true))))