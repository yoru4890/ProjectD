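; Temporary Engineer character child that test-drives grid-based tower and trap building through BuildSystem, using hardcoded keys.
; E readies a MissileTower from build or manage mode; LSM_IA_3 enters manage mode.
; Z and X step towers and thorn traps along row-name upgrade chains; right mouse cancels placed buildings.
; These three check CurrentPlayerMode, while the mode setters write EPlayerMode and both start the build trace.
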(event Input|EnhancedActionEvents|EnhancedInputActionLSM_IA_3
  (params (ActionValue :type Boolean) (ElapsedSeconds :type Float%20%28double-precision%29) (TriggeredSeconds :type Float%20%28double-precision%29) (InputAction :type Input%20Action%20Object%20Reference :default "/Game/0000/LSM/Input/Actions/LSM_IA_3.LSM_IA_3"))
  (:Started
    (CallFunction|SettoManageMode)
    (Development|PrintString "Hello")))

(event Input|EnhancedActionEvents|EnhancedInputActionLSM_IA_LeftMouse
  (params (ActionValue :type Boolean) (ElapsedSeconds :type Float%20%28double-precision%29) (TriggeredSeconds :type Float%20%28double-precision%29) (InputAction :type Input%20Action%20Object%20Reference :default "/Game/0000/LSM/Input/Actions/LSM_IA_LeftMouse.LSM_IA_LeftMouse")))

(event Input|EnhancedActionEvents|EnhancedInputActionLSM_IA_3
  (params (ActionValue :type Boolean) (ElapsedSeconds :type Float%20%28double-precision%29) (TriggeredSeconds :type Float%20%28double-precision%29) (InputAction :type Input%20Action%20Object%20Reference :default "/Game/0000/LSM/Input/Actions/LSM_IA_3.LSM_IA_3")))

(event Input|EnhancedActionEvents|EnhancedInputActionLSM_IA_4
  (params (ActionValue :type Boolean) (ElapsedSeconds :type Float%20%28double-precision%29) (TriggeredSeconds :type Float%20%28double-precision%29) (InputAction :type Input%20Action%20Object%20Reference :default "/Game/0000/LSM/Input/Actions/LSM_IA_4.LSM_IA_4")))

(event EventBeginPlay
  (|CallParentFunction)
  (Class|DDBuildComponent|InitGridBuildManager (Variables|Default|GetBuildSystem)))

(event Collision|EventActorBeginOverlap
  (params (OtherActor :type Actor%20Object%20Reference))
  (|CallParentFunction OtherActor) ; This node is disabled and will not be called.\nDrag off pins to build functionality.
)

(event EventTick
  (params (DeltaSeconds :type Float%20%28single-precision%29))
  (|CallParentFunction DeltaSeconds) ; This node is disabled and will not be called.\nDrag off pins to build functionality.
)

(event Input|MouseEvents|DebugKeyRightMouseButton
  (params (Key :type Key%20Structure :default "None") (ActionValue :type Input%20Action%20Value%20Structure))
  (:Pressed
    (switch Utilities|FlowControl|Switch|SwitchonEPlayerMode (Variables|Default|GetCurrentPlayerMode)
      (:ManagementMode
        (Class|DDBuildComponent|CancelPlacedBuilding (Variables|Default|GetBuildSystem))))))

(event Input|KeyboardEvents|E
  (params (Key :type Key%20Structure :default "None"))
  (:Pressed
    (switch Utilities|FlowControl|Switch|SwitchonLSM_Enum_PlayerMode (Variables|Default|GetEPlayerMode)
      (:NewEnumerator0
        _)
      (:NewEnumerator1
        _))
    (bind _ddbuild (CallFunction|SettoBuildMode))
    (Class|DDBuildComponent|ReadyBuilding _ddbuild (Variables|Default|GetMissileTower))))

(event Input|KeyboardEvents|Z
  (params (Key :type Key%20Structure :default "None"))
  (bind _buildsystem (Variables|Default|GetBuildSystem))
  (:Pressed
    (switch Utilities|FlowControl|Switch|SwitchonEPlayerMode (Variables|Default|GetCurrentPlayerMode)
      (:ManagementMode
        (bind _returnvalue (Class|DDBuildComponent|GetManagedBuildingRowName (Variables|Default|GetBuildSystem)))
        (if (== _returnvalue (Variables|Default|GetMachineGunTower))
          (Class|DDBuildComponent|UpgradeBuilding _buildsystem (Variables|Default|GetUpgradeMachineGunTower))
          (elif (== _returnvalue (Variables|Default|GetUpgradeMachineGunTower))
            (Class|DDBuildComponent|UpgradeBuilding _buildsystem (Variables|Default|GetTankTower))
            (elif (== _returnvalue (Variables|Default|GetTankTower))
              (Class|DDBuildComponent|UpgradeBuilding _buildsystem (Variables|Default|GetUpgradeTankTower)))))))))

(event Input|KeyboardEvents|X
  (params (Key :type Key%20Structure :default "None"))
  (bind _buildsystem (Variables|Default|GetBuildSystem))
  (:Pressed
    (switch Utilities|FlowControl|Switch|SwitchonEPlayerMode (Variables|Default|GetCurrentPlayerMode)
      (:ManagementMode
        (bind _returnvalue (Class|DDBuildComponent|GetManagedBuildingRowName (Variables|Default|GetBuildSystem)))
        (if (== _returnvalue (Variables|Default|GetThornTrap))
          (Class|DDBuildComponent|UpgradeBuilding _buildsystem (Variables|Default|GetUpgradeThornTrap))
          (elif (== _returnvalue (Variables|Default|GetUpgradeThornTrap))
            (Class|DDBuildComponent|UpgradeBuilding _buildsystem (Variables|Default|GetAcidThornTrap))
            (elif (== _returnvalue (Variables|Default|GetAcidThornTrap))
              (Class|DDBuildComponent|UpgradeBuilding _buildsystem (Variables|Default|GetUpgradeAcidThornTrap)))))))))

(event Input|KeyboardEvents|C
  (params (Key :type Key%20Structure :default "None")))

(fn ConstructionScript
  (|CallParentFunction))

(fn SettoBuildMode
  (bind _buildsystem (Variables|Default|GetBuildSystem))
  (Variables|Default|SetEPlayerMode "NewEnumerator0")
  (Class|DDBuildComponent|AllStopTrace _buildsystem)
  (Class|DDBuildComponent|StartBuildTrace _buildsystem)
  (return _buildsystem))

(fn SettoManageMode
  (bind _buildsystem (Variables|Default|GetBuildSystem))
  (Variables|Default|SetEPlayerMode "NewEnumerator1")
  (Class|DDBuildComponent|AllStopTrace _buildsystem)
  (Class|DDBuildComponent|StartBuildTrace _buildsystem))